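; StartFishingBlueprint is a trigger actor that starts fishing when the third-person character overlaps it.
; On overlap, it plays the character's start animation and spawns a fishing rod (CanaPescarBlueprint) owned by that character.
; It snaps the rod to the right-hand socket, applies an offset transform, stores it on the character and calls the character's start-fishing logic.
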(event `self.ReceiveActorBeginOverlap`
  (params (OtherActor :type "Actor Object Reference"))
  (bind _asbp_third_person_character (cast `/Game/ThirdPerson/Blueprints/BP_ThirdPersonCharacter` OtherActor))
  (`/Game/ThirdPerson/Blueprints/BP_ThirdPersonCharacter.StartAnimation` _asbp_third_person_character)
  (bind _mesh (`Character.Mesh` _asbp_third_person_character))
  (bind _returnvalue (`|SpawnActorFromClass` "/Game/Blueprints/CanaPescarBlueprint.CanaPescarBlueprint_C" (`SceneComponent.GetSocketTransform` _mesh "hand_rSocket" "RTS_World") "AlwaysSpawn" "OverrideRootScale" _asbp_third_person_character null))
  (`self.K2_AttachToComponent` _returnvalue _mesh "hand_rSocket" "SnapToTarget" "SnapToTarget" "SnapToTarget" true)
  (`SceneComponent.K2_SetRelativeTransform` (`Actor.RootComponent` _returnvalue) (`self.Offset`) false false)
  (set `/Game/ThirdPerson/Blueprints/BP_ThirdPersonCharacter.Cana` _returnvalue _asbp_third_person_character)
  (`/Game/ThirdPerson/Blueprints/BP_ThirdPersonCharacter.StartFishing` _asbp_third_person_character))

(fn `UserConstructionScript`)
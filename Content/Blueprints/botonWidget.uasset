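; Actor Blueprint, despite the widget name, that moves a Plane component along its relative Z axis at a key-controlled speed.
; Q raises ActualSpeed and prints a debug message, E lowers it, and Tick applies it as a per-frame offset without delta-time scaling.
; Tick zeroes the speed when ClampY matches that offset, but ClampY's clamp math is unused and the clamped SetRelativeLocation never runs.
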(event `self.ReceiveTick`
  (params (DeltaSeconds :type "Float (single-precision)"))
  (bind _returnvalue (* (0.0 0.0 1.0) (`self.actualSpeed`)))
  (`SceneComponent.K2_AddRelativeLocation` (`self.Plane`) _returnvalue false false)
  (if (== (* (`KismetMathLibrary.FClamp` (`self.actualY`) (`self.minY`) (`self.maxY`)) (0.0 0.0 1.0)) _returnvalue)
    (set `self.actualSpeed` 0.0)))

(event `Key|Q`
  (params (Key :type "Key Structure"))
  (:`Pressed`
    (`KismetSystemLibrary.PrintString` "Hello")
    (set `self.actualSpeed` (+ 1.0 (`self.actualSpeed`)))))

(event `Key|E`
  (params (Key :type "Key Structure"))
  (:`Pressed`
    (set `self.actualSpeed` (+ (`self.actualSpeed`) -1.0))))

(fn `UserConstructionScript`)